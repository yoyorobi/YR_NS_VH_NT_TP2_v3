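; BP_Medkit is a floating pickup that changes the player's health on contact.
; Two timelines chain into each other, one forward and one reversed, to loop the mesh's bobbing motion.
; Collision overlap with BP_ThirdPersonCharacter sends HealthChangeAmout to the PlayerState's ACHealth component as healing, or as damage when negative.
; The actor then destroys itself and spawns a Niagara collect effect.
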(event `self.ReceiveBeginPlay`
  (bind _medkit (`self.Medkit`))
  (`SceneComponent.SetVisibility` (`self.NewNiagaraSystem3`) false false)
  (bind (_direction _floating) (`Timeline|Timeline` :!label _label)
    (:`Update`
      (`SceneComponent.K2_SetRelativeLocation` _medkit _floating false false))
    (:`Finished`
      (bind (_direction_2 _floating_2) (`Timeline|Chronologie` :!via `ReverseFromEnd`)
        (:`Update`
          (`SceneComponent.K2_SetRelativeLocation` _medkit _floating_2 false false))
        (:`Finished`
          (goto _label :!via `PlayFromStart`))))))

(event `self.Collision.OnComponentBeginOverlap`
  (params (OverlappedComponent :type "PrimitiveComponent Object Reference") (OtherActor :type "Actor Object Reference") (OtherComp :type "PrimitiveComponent Object Reference") (OtherBodyIndex :type Integer) (bFromSweep :type Boolean) (SweepResult :type "HitResult Structure (by ref)"))
  (bind _asbp_third_person_character (cast `/Game/Game/Blueprints/Pawns_Characters/Player/BP_ThirdPersonCharacter` OtherActor))
  (bind _asbp_player_state (cast `/Game/Game/Blueprints/PlayerStates/BP_PlayerState` (`Pawn.PlayerState` _asbp_third_person_character)))
  (if (< (`self.HealthChangeAmout`) 0.0)
    (bind _ac_health (`/Game/Game/Blueprints/PlayerStates/BP_PlayerState.AC_Health` _asbp_player_state))
    (`/Game/Game/Blueprints/Components/AC_Health.TakeDamage` _ac_health (`KismetMathLibrary.Abs` (`self.HealthChangeAmout`)))
    (else
      (`/Game/Game/Blueprints/Components/AC_Health.GainHealth` _ac_health (`self.HealthChangeAmout`))))
  (`self.K2_DestroyActor`)
  (`NiagaraFunctionLibrary.SpawnSystemAtLocation` "/Game/Game/Blueprints/Actors/SN_Medkit_Collect.SN_Medkit_Collect" (`self.K2_GetActorLocation`)))

(fn `UserConstructionScript`)